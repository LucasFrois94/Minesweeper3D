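; Minesweeper-style block that randomly becomes a mine and builds the field by spawning copies of itself along X and Y, limited by game instance slot counters.
; A timed box trace on a mine-only channel sets each block's colored nearby-mine number or flags it empty.
; Damage reveals numbers and clears adjacent empty blocks.
; Damaged mines explode, signal other mines through a sphere trace, and set game over.
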(fn `CheckBlock`
  (bind _cube (`self.Cube`))
  (bind _returnvalue (`SceneComponent.K2_GetComponentLocation` _cube))
  ;[1 1 1] If the block is empty and around there is none that is checking that some block is indicating that a mine nearby it destroys the empty blocks.
  (bind _outhits (`KismetSystemLibrary.BoxTraceMulti` :`Start` _returnvalue :`End` (+ _returnvalue (* (`SceneComponent.GetForwardVector` _cube) 1.0)) :`HalfSize` (110.0 110.0 110.0) :`TraceChannel` "TraceTypeQuery3" :`TraceColor` (struct :`R` 1.0 :`G` 0.988119 :`A` 1.0) :`TraceHitColor` (struct :`G` 1.0 :`B` 1.0 :`A` 1.0) :`DrawTime` 1.0))
  (for _array_element _outhits
    (bind (_bblockinghit _binitialoverlap _time _distance _location _impactpoint _normal _impactnormal _physmat _hitactor) (`GameplayStatics.BreakHitResult` _array_element))
    (if _bblockinghit
      (bind _asblock_bp (cast `/Game/Blueprints/Block/Block_BP` _hitactor))
      (`/Engine/EditorBlueprintResources/StandardMacros.IsValid` _asblock_bp
        (:`Is Valid`
          (if (and (`/Game/Blueprints/Block/Block_BP.IsEmpty` _asblock_bp) (not (`/Game/Blueprints/Block/Block_BP.IsMine` _asblock_bp)))
            (`self.K2_DestroyActor` _hitactor)
            (`self.IfBlockEmpty`
              (:`true`
                (`self.K2_DestroyActor`)))))))))

(fn `CheckMine`
  (bind _cubenumber (`self.CubeNumber`))
  (bind _color3 (`self.Color3`))
  (bind _cube (`self.Cube`))
  (bind _returnvalue (`SceneComponent.K2_GetComponentLocation` _cube))
  ;[1 1 1] Check for a mine nearby and set the amount of mines around that block clicked
  (`self.IsVerifedMacro`
    (:`else`
      (bind (_outhits _returnvalue_2) (`KismetSystemLibrary.BoxTraceMulti` :`Start` _returnvalue :`End` (+ _returnvalue (* (`SceneComponent.GetForwardVector` _cube) 1.0)) :`HalfSize` (110.0 110.0 110.0) :`TraceChannel` "TraceTypeQuery4" :`TraceColor` (struct :`R` 1.0 :`B` 0.005584 :`A` 1.0) :`TraceHitColor` (struct :`R` 0.331466 :`G` 1.0 :`A` 1.0) :`DrawTime` 1.0))
      ;;[0.3698 0 0.1875] If a block is empty
      (if (not _returnvalue_2)
        (set `self.IsEmpty` true))
      (set `self.IsVerified` true)
      (for (_array_element _array_index) _outhits
        (bind (_bblockinghit _binitialoverlap _time _distance _location _impactpoint _normal _impactnormal _physmat _hitactor) (`GameplayStatics.BreakHitResult` _array_element))
        (if _bblockinghit
          (bind _asblock_bp (cast `/Game/Blueprints/Block/Block_BP` _hitactor))
          (`/Engine/EditorBlueprintResources/StandardMacros.IsValid` _asblock_bp
            (:`Is Valid`
              (bind _output_get (set `self.Index` (+ _array_index 1)))
              (`TextRenderComponent.K2_SetText` _cubenumber (`KismetTextLibrary.Conv_StringToText` (`KismetStringLibrary.Conv_IntToString` _output_get)))
              (`TextRenderComponent.SetTextRenderColor` _cubenumber (select `int` (`self.Index`) :`0` (struct) :`1` (`self.Color1`) :`2` (`self.Color2`) :`3` _color3 :`4` _color3 :`5` _color3))
              (set `self.MineIsClose` true))))))))

(fn `IfSelfBlockEmpty`
  (`self.IfBlockEmpty`
    (:`false`
      (`SceneComponent.SetHiddenInGame` (`self.CubeNumber`) false false))))

(fn `KillemAll`
  (bind _returnvalue (`self.K2_GetActorLocation`))
  ;[1 1 1] Check if a mine is exploded all existing mines in the field will explode
  (`self.IsMineMacro`
    (:`True`
      (bind _outhits (`KismetSystemLibrary.SphereTraceMulti` _returnvalue (+ _returnvalue (* (`self.GetActorForwardVector`) 0.0)) 1000.0 "TraceTypeQuery3"))
      (for _array_element _outhits
        (bind (_bblockinghit _binitialoverlap _time _distance _location _impactpoint _normal _impactnormal _physmat _hitactor) (`GameplayStatics.BreakHitResult` _array_element))
        (if _bblockinghit
          (bind _asblock_bp (cast `/Game/Blueprints/Block/Block_BP` _hitactor))
          (if (`/Game/Blueprints/Block/Block_BP.IsMine` _asblock_bp)
            (`self.Explosion` _asblock_bp)))))))

(fn `UserConstructionScript`
  (bind _returnvalue (`PrimitiveComponent.CreateDynamicMaterialInstance` (`self.Cube`) 0 "/Engine/BasicShapes/Basic_Square_Outline_Mat_Inst.Basic_Square_Outline_Mat_Inst" "None"))
  (set `self.Mat_Ref` _returnvalue))