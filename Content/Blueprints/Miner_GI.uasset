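; Miner_GI holds shared state for a mining game, tracking game over and block placement limits along the X and Y axes.
; AddSideSlot and AddDownSlot increment counters and flag each direction as full past a fixed limit.
; SetGameOver, gated by a GameOver check macro, disables player input, resets slot state, then shows a new Game_UI widget after a delay.
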(event `SetGameOver`
  ;[1 0 0] Set Game Over Functions
  (`self.GameOverMacro`
    (:`else`
      (set `self.GameOver` true)
      (`Actor.DisableInput` (`GameplayStatics.GetPlayerPawn` 0) (`GameplayStatics.GetPlayerController` 0))
      (set `self.SideSlots` 0)
      (set `self.DownSlots` 0)
      (set `self.FullSideSlot` false)
      (set `self.FullDownSlot` false)
      (`KismetSystemLibrary.Delay` 5.0)
      (bind _returnvalue (`|CreateWidget` "/Game/Blueprints/UI/Game_UI.Game_UI_C"))
      (`UserWidget.AddToViewport` _returnvalue 0))))

(fn `AddDownSlot`
  ;[0 1 0.913] check the amount of blocks added at Y position to limit
  (bind _output_get (set `self.DownSlots` (+ (`self.DownSlots`) 1)))
  (if (> _output_get 9)
    (set `self.FullDownSlot` true)))

(fn `AddSideSlot`
  ;[0 1 0.9873] check the amount of blocks added at x position to limit
  (bind _output_get (set `self.SideSlots` (+ (`self.SideSlots`) 1)))
  (if (> _output_get 90)
    (set `self.FullSideSlot` true)))